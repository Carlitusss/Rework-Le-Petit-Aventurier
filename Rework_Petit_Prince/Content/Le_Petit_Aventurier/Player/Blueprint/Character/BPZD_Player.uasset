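; BPZD_Player is the player character Blueprint, handling Enhanced Input setup and basic movement.
; On BeginPlay it adds the IMC_General mapping context through the player controller's local player subsystem, printing an error if that subsystem is invalid.
; IA_Move feeds movement input along fixed world axes, X to world Y (right/left) and Y to world X (front/back), independent of camera or control rotation.
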(event `self.ReceiveBeginPlay`
  ;[1 1 1 0.5] Event Begin Play
  (bind _asplayer_controller (cast `PlayerController` (`self.GetController`)))
  (bind _returnvalue (pcsubsystem `EnhancedInputLocalPlayerSubsystem` _asplayer_controller))
  (`/Engine/EditorBlueprintResources/StandardMacros.IsValid` _returnvalue
    (:`Is Valid`
      (`EnhancedInputSubsystemInterface.AddMappingContext` _returnvalue "/Game/Le_Petit_Aventurier/Player/Blueprint/Inputs/IMC_General.IMC_General" 0 (struct)))
    (:`Is Not Valid`
      (`KismetSystemLibrary.PrintString` "Enhanced Input Local Player Subsystem ERROE" true true (struct :`R` 1.0 :`G` 0.100087 :`A` 1.0)))))

(event `EnhancedInput|/Game/Input/Actions/IA_Move`
  (params (ActionValue :type "Vector2D Structure") (ElapsedSeconds :type "Float (double-precision)") (TriggeredSeconds :type "Float (double-precision)") (InputAction :type "InputAction Object Reference" :default "/Game/Input/Actions/IA_Move.IA_Move"))
  (bind (_x _y) (`KismetMathLibrary.BreakVector2D` ActionValue))
  ;[1 1 1 0.5] Movement
  (:`Triggered`
    ;;[0.005208 0.005208 0.005208 0.5] Right / Left
    (`self.AddMovementInput` (0.0 1.0 0.0) _x)
    ;;[0.005208 0.005208 0.005208 0.5] Front / Back
    (`self.AddMovementInput` (1.0 0.0 0.0) _y)))

(fn `UserConstructionScript`)